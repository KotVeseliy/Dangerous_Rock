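; Actor component that tracks its owner's health and signals when it runs out.
; On BeginPlay it binds to the owner's OnTakeAnyDamage event and initializes Health from DefaultHealth.
; Damage lowers Health, clamped between zero and its current value, and each hit that leaves it at zero calls the OnOwnerDied dispatcher.
; Getters expose both values, while SetDefaultHealth has an empty body.
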(event Custom|OnTakeAnyDamage_Event
  (params (DamagedActor :type Actor%20Object%20Reference) (Damage :type Float%20%28single-precision%29) (DamageType :type Damage%20Type%20Object%20Reference) (InstigatedBy :type Controller%20Object%20Reference) (DamageCauser :type Actor%20Object%20Reference))
  (bind _health (Variables|Default|GetHealth))
  (CallFunction|SetHealth (Math|Float|Clamp(Float) (- _health Damage) 0.0 _health))
  (if (<= (CallFunction|GetHealth) 0.0)
    (Default|CallOnOwnerDied)))

(event EventBeginPlay
  (EventDispatchers|AssignOnTakeAnyDamage (Components|GetOwner) (delegate Custom|OnTakeAnyDamage_Event))
  (CallFunction|SetHealth (Variables|Default|GetDefaultHealth)))

(fn SetHealth
  (params (Health :type Float%20%28double-precision%29))
  (Variables|Default|SetHealth Health))

(fn GetHealth
  (return (Variables|Default|GetHealth)))

(fn SetDefaultHealth)

(fn GetDefaultHealth
  (return (Variables|Default|GetDefaultHealth)))