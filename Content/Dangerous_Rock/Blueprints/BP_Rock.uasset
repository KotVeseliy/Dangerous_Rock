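; BP_Rock is a moving hazard actor that launches toward the player and damages them on contact.
; On BeginPlay it rotates to face player pawn 0 and binds its hit event.
; Tick sweeps it along the X and Y of its forward vector at Speed.
; Hitting a "Player"-tagged actor applies damage and destroys the rock; any other hit bounces it by reflecting its heading off the surface normal, using yaw only.
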(event Custom|OnActorHit_Event
  (params (SelfActor :type Actor%20Object%20Reference) (OtherActor :type Actor%20Object%20Reference) (NormalImpulse :type Vector) (Hit :type Hit%20Result%20Structure%20%28by%20ref%29))
  (if (Actor|ActorHasTag OtherActor "Player")
    (Game|Damage|ApplyDamage OtherActor (Variables|Default|GetBase%20Damage) 0 self)
    (Actor|DestroyActor)
    (else
      (Transformation|SetActorRotation (Math|Rotator|MakeRotator 0.0 0.0 (.yaw (Math|Rotator|MakeRotfromX (Math|Vector|GetReflectionVector (Transformation|GetActorForwardVector) (.Normal (Collision|BreakHitResult Hit))))))))))

(event EventTick
  (params (DeltaSeconds :type Float%20%28single-precision%29))
  (bind _returnvalue (Transformation|GetActorForwardVector))
  (bind _speed (Variables|Gameplay|GetSpeed))
  (bind _returnvalue_2 (* DeltaSeconds _speed))
  (bind _returnvalue_3 (* _returnvalue_2 _returnvalue))
  (Transformation|AddActorWorldOffset (Math|Vector|MakeVector (.x _returnvalue_3) (.y _returnvalue_3) 0.0) true))

(event EventBeginPlay
  (Utilities|FlowControl|Sequence
    (:then_0
      (Utilities|TurntoPlayer))
    (:then_1
      (EventDispatchers|BindEventtoOnActorHit (EventDispatchers|CreateEvent :!event Custom|OnActorHit_Event)))))

(fn ConstructionScript)