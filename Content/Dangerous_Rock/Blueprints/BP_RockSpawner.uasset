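; BP_RockSpawner periodically spawns BP_Rock hazards at random positions within its Box volume.
; On BeginPlay it reads the difficulty from BP_DangerousRockGameInstance to set rock damage and the interval of a looping spawn timer.
; Each tick of that timer picks random X and Y inside the box, keeps the spawner's Z, and passes the damage to the new rock.
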(event Custom|SpawnRockInVolume
  (bind _box (Variables|Default|GetBox))
  (bind _returnvalue (Transformation|GetWorldLocation _box))
  (bind _returnvalue_2 (Components|Box|GetScaledBoxExtent _box))
  (bind _returnvalue_3 (Math|Random|RandomPointinBoundingBox _returnvalue _returnvalue_2))
  (bind (_x _y) (Math|Vector|BreakVector _returnvalue_3))
  (Game|SpawnActorfromClass "/Game/Dangerous_Rock/Blueprints/BP_Rock.BP_Rock_C" (Math|Transform|MakeTransform (Math|Vector|MakeVector _x _y (.Z (Math|Vector|BreakVector (Transformation|GetActorLocation))))) "AdjustIfPossibleButAlwaysSpawn" 0 (Variables|Default|GetBaseRockDammage) 0))

(event EventBeginPlay
  (bind _asbp_dangerous_rock_game_instance (Utilities|Casting|CastToBP_DangerousRockGameInstance (Game|GetGameInstance)))
  (Variables|Default|SetBaseRockDammage (Utilities|Select :Index (Default|GetGameDifficulty _asbp_dangerous_rock_game_instance) :NewEnumerator0 25.0 :NewEnumerator1 34.0 :NewEnumerator2 5e+01))
  (Utilities|Time|SetTimerbyEvent (delegate Custom|SpawnRockInVolume) (Utilities|Select :Index (Default|GetGameDifficulty _asbp_dangerous_rock_game_instance) :NewEnumerator0 3.0 :NewEnumerator1 2.0 :NewEnumerator2 1.0) true))

(fn ConstructionScript)